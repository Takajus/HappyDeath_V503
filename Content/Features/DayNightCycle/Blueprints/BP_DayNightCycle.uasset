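; Day/night cycle Blueprint that alternates a Sun and a Moon light in an endless loop from BeginPlay.
; Two chained Timelines drive the pitch of each light actor in turn, with the night Timeline restarting the day one.
; Each phase reveals the other light when its value reaches a threshold, then on finish hides its own light and toggles IsDay.
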(event `self.ReceiveBeginPlay`
  ;[1 0.7402 0.1297] DayCycle
  (bind (_direction _day__value) (`Timeline|Timeline_0` :!label _label)
    (:`Update`
      (bind _output_get (set `self.day%Value` _day__value))
      (if (<= _output_get -0.98)
        (`SceneComponent.SetVisibility` (`Light.LightComponent` (`self.Moon`)) true false))
      (`self.K2_SetActorRotation` (`self.Sun`) (`KismetMathLibrary.MakeRotator` 0.0 (* (`self.day%Value`) 180.0) 0.0) false))
    (:`Finished`
      (set `self.isDay` (not (`self.isDay`)))
      (`SceneComponent.SetVisibility` (`Light.LightComponent` (`self.Sun`)) false false)
      ;[0.4984 0.4255 1] NightCycle
      (bind (_direction_2 _night__value) (`Timeline|Timeline_1` :!via `PlayFromStart`)
        (:`Update`
          (bind _output_get_2 (set `self.night% Value` _night__value))
          (if (<= _output_get_2 -0.98)
            (`SceneComponent.SetVisibility` (`Light.LightComponent` (`self.Sun`)) true false))
          (`self.K2_SetActorRotation` (`self.Moon`) (`KismetMathLibrary.MakeRotator` 0.0 (* (`self.night% Value`) 180.0)) false))
        (:`Finished`
          (set `self.isDay` (not (`self.isDay`)))
          (`SceneComponent.SetVisibility` (`Light.LightComponent` (`self.Moon`)) false false)
          (`self.RestartCycle`))))))

(event `RestartCycle`
  ;[1 0.7402 0.1297] DayCycle
  (goto _label :!via `PlayFromStart`))

(fn `UserConstructionScript`)
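; Bp_Dig is a diggable dynamic-mesh actor that has a hole cut into it on interaction, using Geometry Script.
; The construction script resets the mesh and appends a box below the origin.
; Interact calls AddHole, which subtracts a slightly offset box at a fixed location using a pooled compute mesh, then releases the pool.
; Timed and randomized digging logic is left unconnected.
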(event `self.ReceiveBeginPlay`)

(event `/Game/Features/Interactions/Component/BPI_Interactable.Interact`
  (`self.AddHole`))

(event `self.ReceiveTick`
  (params (DeltaSeconds :type "Float (single-precision)")))

(fn `AddHole`
  (bind _returnvalue (`self.AllocateComputeMesh`))
  (bind _returnvalue_2 (`GeometryScriptLibrary_MeshPrimitiveFunctions.AppendBox` _returnvalue (struct) (`KismetMathLibrary.MakeTransform` (0.0 0.0 -119.0)) 100.0 100.0 100.0 0 0 0 "Base" null))
  (bind _returnvalue_3 (`BaseDynamicMeshComponent.GetDynamicMesh` (`self.DynamicMeshComponent`)))
  (`GeometryScriptLibrary_MeshBooleanFunctions.ApplyMeshBoolean` _returnvalue_3 (struct) _returnvalue_2 (struct) "Subtract" (struct) null)
  (`self.ReleaseAllComputeMeshes`))

(fn `UserConstructionScript`
  (bind _returnvalue (`BaseDynamicMeshComponent.GetDynamicMesh` (`self.DynamicMeshComponent`)))
  (bind _returnvalue_2 (`DynamicMesh.Reset` _returnvalue))
  (`GeometryScriptLibrary_MeshPrimitiveFunctions.AppendBox` _returnvalue_2 (struct) (`KismetMathLibrary.MakeTransform` (0.0 0.0 -120.0)) 100.0 100.0 100.0 0 0 0 "Base" null))
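; BP_InteractionExample is a sample interactable actor that demonstrates the interaction feature's hover and interact events.
; Interact and EndInteraction switch the CubeInteract mesh between InteractMat and BaseMat, while Hover and UnHover switch CubeHover between HoverMat and BaseMat.
; Each event also prints a debug message containing the actor's display name.
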(event `/Game/Features/Interactions/Component/BPI_Interactable.Interact`
  (`KismetSystemLibrary.PrintString` (`KismetStringLibrary.Concat_StrStr` "Interacted with : " (`KismetSystemLibrary.GetDisplayName` self)))
  (`PrimitiveComponent.SetMaterial` (`self.CubeInteract`) 0 (`self.InteractMat`)))

(event `/Game/Features/Interactions/Component/BPI_Interactable.EndInteraction`
  (`KismetSystemLibrary.PrintString` (`KismetStringLibrary.Concat_StrStr` "End interaction with : " (`KismetSystemLibrary.GetDisplayName` self)))
  (`PrimitiveComponent.SetMaterial` (`self.CubeInteract`) 0 (`self.BaseMat`)))

(event `/Game/Features/Interactions/Component/BPI_Interactable.Hover`
  (`KismetSystemLibrary.PrintString` (`KismetStringLibrary.Concat_StrStr` "Hover : " (`KismetSystemLibrary.GetDisplayName` self)))
  (`PrimitiveComponent.SetMaterial` (`self.CubeHover`) 0 (`self.HoverMat`)))

(event `/Game/Features/Interactions/Component/BPI_Interactable.UnHover`
  (`KismetSystemLibrary.PrintString` (`KismetStringLibrary.Concat_StrStr` "UnHover  : " (`KismetSystemLibrary.GetDisplayName` self)))
  (`PrimitiveComponent.SetMaterial` (`self.CubeHover`) 0 (`self.BaseMat`)))

(fn `UserConstructionScript`)
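; BP_InteractionExample_Child is an example interactable actor that shows feedback for the interaction system's hover and interact events.
; Hover and UnHover swap the CubeHover material between hover and base materials.
; Interact and EndInteraction do the same on CubeInteract with the interact and base materials.
; Each event also prints a message with the actor's display name; the construction script only calls its parent.
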(event `/Game/Features/Interactions/Component/BPI_Interactable.Interact`
  (`KismetSystemLibrary.PrintString` (`KismetStringLibrary.Concat_StrStr` "Interacted with : " (`KismetSystemLibrary.GetDisplayName` self)))
  (`PrimitiveComponent.SetMaterial` (`self.CubeInteract`) 0 (`self.InteractMaterial`)))

(event `/Game/Features/Interactions/Component/BPI_Interactable.EndInteraction`
  (`KismetSystemLibrary.PrintString` (`KismetStringLibrary.Concat_StrStr` "End interaction with : " (`KismetSystemLibrary.GetDisplayName` self)))
  (`PrimitiveComponent.SetMaterial` (`self.CubeInteract`) 0 (`self.BaseMaterial`)))

(event `/Game/Features/Interactions/Component/BPI_Interactable.Hover`
  (`KismetSystemLibrary.PrintString` (`KismetStringLibrary.Concat_StrStr` "Hover : " (`KismetSystemLibrary.GetDisplayName` self)))
  (`PrimitiveComponent.SetMaterial` (`self.CubeHover`) 0 (`self.HoverMaterial`)))

(event `/Game/Features/Interactions/Component/BPI_Interactable.UnHover`
  (`KismetSystemLibrary.PrintString` (`KismetStringLibrary.Concat_StrStr` "UnHover  : " (`KismetSystemLibrary.GetDisplayName` self)))
  (`PrimitiveComponent.SetMaterial` (`self.CubeHover`) 0 (`self.BaseMaterial`)))

(fn `UserConstructionScript`
  (`parent.UserConstructionScript`))
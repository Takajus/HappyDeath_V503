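; Building placement component that lets the player position and rotate an actor on BP_Tile tiles.
; SelectBuilding toggles a preview, spawning it below the pawn or destroying the current one, with Tab as a test trigger for BP_Build.
; PlaceHandler snaps the preview to the tile under the cursor via a trace and applies the stored yaw.
; R rotates in 90-degree steps, and IA_Interact confirms placement by releasing the reference.
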(event `PlaceHandler`
  (bind (_placementrotation_x _placementrotation_y _placementrotation_z) (`KismetMathLibrary.BreakVector` (`self.PlacementRotation`)))
  (bind _asbp_tile (cast `/Game/Features/Grid/Blueprint/BP_Tile` (`.HitActor` (`GameplayStatics.BreakHitResult` (`PlayerController.GetHitResultUnderCursorByChannel` (`GameplayStatics.GetPlayerController` 0) "TraceTypeQuery3" true)))))
  (`Actor.K2_SetActorLocation` (`self.ActorToPlace`) (`Actor.K2_GetActorLocation` _asbp_tile) false false)
  (`Actor.K2_SetActorRotation` (`self.ActorToPlace`) (`KismetMathLibrary.MakeRotator` 0.0 0.0 _placementrotation_z) false))

(event `Key|Tab`
  (params (Key :type "Key Structure"))
  ;[0.05127 0.05127 0.05127] Test for object placing
  (:`Pressed`
    (`self.SelectBuilding` "/Game/Features/Interactions/Blueprint/BP_Build.BP_Build_C")))

(event `Key|R`
  (params (Key :type "Key Structure"))
  ;[0.05127 0.05127 0.05127] Test for object placing
  (:`Pressed`
    (bind _result (`self.Is Placing ?`))
    (if _result
      (set `self.PlacementRotation` (+ (`self.PlacementRotation`) (0.0 0.0 90.0))))))

(event `EnhancedInput|/Game/Features/Character/Input/Actions/IA_Interact`
  (params (ActionValue :type "Float (double-precision)") (ElapsedSeconds :type "Float (double-precision)") (TriggeredSeconds :type "Float (double-precision)") (InputAction :type "InputAction Object Reference" :default "/Game/Features/Character/Input/Actions/IA_Interact.IA_Interact"))
  ;[0.05127 0.05127 0.05127] Test for object placing
  (:`Started`
    (bind _result (`self.Is Placing ?`))
    (if _result
      (set `self.ActorToPlace` null))))

(fn `Is Placing ?`
  (returns (result :type Boolean))
  (if (== (`self.ActorToPlace`) null)
    (return false)
    (else
      (return true))))

(fn `SelectBuilding`
  (params (ActorToPlace :type "Actor Class Reference"))
  (bind (_returnvalue_x _returnvalue_y) (`KismetMathLibrary.BreakVector` (`Actor.K2_GetActorLocation` (`GameplayStatics.GetPlayerPawn` 0))))
  (if (== (`self.ActorToPlace`) null)
    (bind _returnvalue (`|SpawnActorFromClass` ActorToPlace (`KismetMathLibrary.MakeTransform` (`KismetMathLibrary.MakeVector` _returnvalue_x _returnvalue_y -200.0)) "Undefined" "OverrideRootScale" null null))
    (set `self.ActorToPlace` _returnvalue)
    (set `self.PlacementRotation` (0.0 0.0 0.0))
    (else
      (`Actor.K2_DestroyActor` (`self.ActorToPlace`))
      (set `self.ActorToPlace` null))))
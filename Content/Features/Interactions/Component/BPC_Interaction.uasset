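; Interaction component that lets the player hover and interact with BPI_Interactable actors through two targeting channels, mouse cursor and sphere trace.
; Both traces run every tick and send hover and unhover messages, holding back unhover while both share a target.
; The sign of IA_Interact's value picks the sphere or mouse target, then toggles or switches the interaction.
; Losing hover on the active target ends its interaction.
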(event `Mouse Detection`
  (bind (_hitresult _returnvalue) (`PlayerController.GetHitResultUnderCursorByChannel` (`GameplayStatics.GetPlayerController` 0) "TraceTypeQuery1" true))
  ;[0.05127 0.05127 0.05127] Mouse object detection
  (if _returnvalue
    (if (`KismetSystemLibrary.DoesImplementInterface` (`.HitActor` (`GameplayStatics.BreakHitResult` _hitresult)) "/Game/Features/Interactions/Component/BPI_Interactable.BPI_Interactable_C")
      (if (not (== (`.HitActor` (`GameplayStatics.BreakHitResult` _hitresult)) (`self.Mouse Targeted Interactable`)))
        (`self.UnSelect` true (`self.Mouse Targeted Interactable`))
        (bind _output_get (set `self.Mouse Targeted Interactable` (`.HitActor` (`GameplayStatics.BreakHitResult` _hitresult))))
        (message `/Game/Features/Interactions/Component/BPI_Interactable.Hover` _output_get))
      (else
        (`self.UnSelect` true (`self.Mouse Targeted Interactable`))))
    (else
      (`self.UnSelect` true (`self.Mouse Targeted Interactable`)))))

(event `Collider Detection`
  (bind _playerpawn (`self.PlayerPawn`))
  (bind _returnvalue (+ (`Actor.K2_GetActorLocation` _playerpawn) (* (`Actor.GetActorForwardVector` _playerpawn) (50.0 50.0 50.0))))
  ;[0.05127 0.05127 0.05127] Object detection
  (bind (_outhit _returnvalue_2) (`KismetSystemLibrary.SphereTraceSingle` :`Start` _returnvalue :`End` (+ _returnvalue (* (`Actor.GetActorUpVector` _playerpawn) (-40.0 -40.0 -40.0))) :`Radius` (`self.Interaction Radius`) :`TraceChannel` "TraceTypeQuery1" :`DrawDebugType` "ForOneFrame" :`DrawTime` 0.3))
  (if _returnvalue_2
    (if (`KismetSystemLibrary.DoesImplementInterface` (`.HitActor` (`GameplayStatics.BreakHitResult` _outhit)) "/Game/Features/Interactions/Component/BPI_Interactable.BPI_Interactable_C")
      (if (not (== (`.HitActor` (`GameplayStatics.BreakHitResult` _outhit)) (`self.Targeted Interactable`)))
        (`self.UnSelect` false (`self.Targeted Interactable`))
        (bind _output_get (set `self.Targeted Interactable` (`.HitActor` (`GameplayStatics.BreakHitResult` _outhit))))
        (message `/Game/Features/Interactions/Component/BPI_Interactable.Hover` _output_get))
      (else
        (`self.UnSelect` false (`self.Targeted Interactable`))))
    (else
      (`self.UnSelect` false (`self.Targeted Interactable`)))))

(event `UnSelect`
  (params (isMouseInput :type Boolean) (ActorToUnSelect :type "Actor Object Reference"))
  ;[0.05127 0.05127 0.05127] Object detection
  ;;[0.05127 0.05127 0.05127] UnSelect the current TargetedInteractable if valid
  (if (== (`self.Mouse Targeted Interactable`) (`self.Targeted Interactable`))
    (if isMouseInput
      (set `self.Mouse Targeted Interactable` null)
      (else
        (set `self.Targeted Interactable` null)))
    (elif isMouseInput
      (`self.HandleUnSelect` ActorToUnSelect)
      (set `self.Mouse Targeted Interactable` null)
      (else
        (`self.HandleUnSelect` ActorToUnSelect)
        (set `self.Targeted Interactable` null)))))

(event `EnhancedInput|/Game/Features/Character/Input/Actions/IA_Interact`
  (params (ActionValue :type "Float (double-precision)") (ElapsedSeconds :type "Float (double-precision)") (TriggeredSeconds :type "Float (double-precision)") (InputAction :type "InputAction Object Reference" :default "/Game/Features/Character/Input/Actions/IA_Interact.IA_Interact"))
  ;[0.05127 0.05127 0.05127] Object detection
  ;;[0.05127 0.05127 0.05127] Interact
  (:`Started`
    (if (>= ActionValue 0.0)
      (`self.HandleSelection` (`self.Targeted Interactable`))
      (else
        (`self.HandleSelection` (`self.Mouse Targeted Interactable`))))))

(event `self.ReceiveTick`
  (params (DeltaSeconds :type "Float (single-precision)"))
  ;[0.05127 0.05127 0.05127] Object detection
  ;;[0.05127 0.05127 0.05127] Every Frame
  (`|ExecutionSequence`
    (:`then_0`
      (`self.Mouse Detection`))
    (:`then_1`
      (`self.Collider Detection`))))

(fn `HandleSelection`
  (params (InputObject :type "Actor Object Reference"))
  (if (== (`self.Interacted`) InputObject)
    (`/Engine/EditorBlueprintResources/StandardMacros.IsValid` InputObject
      (:`Is Valid`
        (if (`self.Is Interacting`)
          (set `self.Is Interacting` false)
          (message `/Game/Features/Interactions/Component/BPI_Interactable.EndInteraction` (`self.Interacted`))
          (set `self.Interacted` null)
          (else
            (set `self.Is Interacting` true)
            (message `/Game/Features/Interactions/Component/BPI_Interactable.Interact` InputObject)
            (set `self.Interacted` InputObject)))))
    (else
      (`/Engine/EditorBlueprintResources/StandardMacros.IsValid` InputObject
        (:`Is Valid`
          (if (`self.Is Interacting`)
            (message `/Game/Features/Interactions/Component/BPI_Interactable.EndInteraction` (`self.Interacted`))
            (bind _output_get (set `self.Interacted` InputObject))
            (message `/Game/Features/Interactions/Component/BPI_Interactable.Interact` _output_get)
            (else
              (set `self.Is Interacting` true)
              (message `/Game/Features/Interactions/Component/BPI_Interactable.Interact` InputObject)
              (set `self.Interacted` InputObject))))))))

(fn `HandleUnSelect`
  (params (ObjectToUnSelect :type "Actor Object Reference"))
  (`/Engine/EditorBlueprintResources/StandardMacros.IsValid` ObjectToUnSelect
    (:`Is Valid`
      (message `/Game/Features/Interactions/Component/BPI_Interactable.UnHover` ObjectToUnSelect)
      (if (and (`self.Is Interacting`) (== ObjectToUnSelect (`self.Interacted`)))
        (message `/Game/Features/Interactions/Component/BPI_Interactable.EndInteraction` (`self.Interacted`))
        (set `self.Is Interacting` false)
        (set `self.Interacted` null))
      (return))))
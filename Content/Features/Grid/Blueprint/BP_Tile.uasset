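; BP_Tile is an interactable grid tile that highlights on hover and can be dug.
; On BeginPlay it spawns a Bp_Dig actor at its own location and keeps a reference to it.
; Hover and UnHover swap the cube's material between hover and base, while Interact delegates digging to that actor through AddHole.
; EndInteraction is left empty.
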(event `self.ReceiveBeginPlay`
  (bind _returnvalue (`|SpawnActorFromClass` "/Game/Features/Dig/Blueprints/Bp_Dig.Bp_Dig_C" (`KismetMathLibrary.MakeTransform` (`self.K2_GetActorLocation`)) "Undefined" "OverrideRootScale" null null))
  (set `self.m_BP_Dig` _returnvalue))

(event `/Game/Features/Interactions/Component/BPI_Interactable.Hover`
  (`PrimitiveComponent.SetMaterial` (`self.Cube`) 0 (`self.M_Hover`)))

(event `/Game/Features/Interactions/Component/BPI_Interactable.Interact`
  (`/Game/Features/Dig/Blueprints/Bp_Dig.AddHole` (`self.m_BP_Dig`)))

(event `/Game/Features/Interactions/Component/BPI_Interactable.UnHover`
  (`PrimitiveComponent.SetMaterial` (`self.Cube`) 0 (`self.M_Base`)))

(event `/Game/Features/Interactions/Component/BPI_Interactable.EndInteraction`)

(fn `UserConstructionScript`)
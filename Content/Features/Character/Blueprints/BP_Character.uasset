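; Player character Blueprint that owns the inventory widget and handles interaction with nearby objects.
; BeginPlay creates and stores the InventoryWG widget, briefly adding it to the viewport to call AddToInventoryMapChange before removing it.
; The I key uses a FlipFlop to show or hide the inventory, switching mouse cursor and input mode with it.
; The E key sends InteractMessage to the first overlapping actor that implements BPI_Interactable.
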(event `self.ReceiveBeginPlay`
  (bind _returnvalue (`|CreateWidget` "/Game/Features/Inventory/UI/InventoryWG.InventoryWG_C"))
  (bind _output_get (set `self.InventoryWG` _returnvalue))
  (`UserWidget.AddToViewport` _output_get 0)
  (`/Game/Features/Inventory/UI/InventoryWG.AddToInventory(MapChange)` :`self` _output_get)
  (`Widget.RemoveFromParent` _output_get))

(event `Key|I`
  (params (Key :type "Key Structure"))
  (bind _returnvalue (`GameplayStatics.GetPlayerController` 0))
  (bind _inventorywg (`self.InventoryWG`))
  ;[1 1 1] Open Inventory UI
  (:`Pressed`
    (`/Engine/EditorBlueprintResources/StandardMacros.FlipFlop`
      (:`A`
        (`UserWidget.AddToViewport` _inventorywg 0)
        (set `PlayerController.bShowMouseCursor` true _returnvalue)
        (`WidgetBlueprintLibrary.SetInputMode_GameAndUIEx` _returnvalue (`self.InventoryWG`)))
      (:`B`
        (`Widget.RemoveFromParent` _inventorywg)
        (set `PlayerController.bShowMouseCursor` false _returnvalue)
        (`WidgetBlueprintLibrary.SetInputMode_GameOnly` _returnvalue)))))

(event `Key|E`
  (params (Key :type "Key Structure"))
  ;[1 1 1] Interact With Objects Inventory
  (:`Pressed`
    (for _array_element (`self.GetOverlappingActors` "/Script/Engine.Actor")
      (if (`KismetSystemLibrary.DoesImplementInterface` _array_element "/Game/Features/Interactions/Component/BPI_Interactable.BPI_Interactable_C")
        (message `/Game/Features/Interactions/Component/BPI_Interactable.Interact` _array_element)
        (break)))))

(fn `UserConstructionScript`)
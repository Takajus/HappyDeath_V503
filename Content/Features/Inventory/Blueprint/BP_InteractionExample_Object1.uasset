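; Example interactable pickup actor for the inventory feature that reacts to hover and interaction.
; Hover and interaction events print debug messages and swap materials on separate hover and interact cubes.
; Interact also casts the player to BP_Character, passes ItemInfo to its InventoryWG widget via AddToInventory, then destroys the actor.
; UseItem is a placeholder that only prints a message.
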(event `/Game/Features/Interactions/Component/BPI_Interactable.Interact`
  (`KismetSystemLibrary.PrintString` (`KismetStringLibrary.Concat_StrStr` "Interacted with : " (`KismetSystemLibrary.GetDisplayName` self)))
  (`PrimitiveComponent.SetMaterial` (`self.CubeInteract`) 0 (`self.InteractMaterial`))
  (bind _asbp_character (cast `/Game/Features/Character/Blueprints/BP_Character` (`GameplayStatics.GetPlayerCharacter` 0)))
  (`/Game/Features/Inventory/UI/InventoryWG.AddToInventory` (`/Game/Features/Character/Blueprints/BP_Character.InventoryWG` _asbp_character) (`self.Item_Info`))
  (`self.K2_DestroyActor`))

(event `/Game/Features/Interactions/Component/BPI_Interactable.EndInteraction`
  (`KismetSystemLibrary.PrintString` (`KismetStringLibrary.Concat_StrStr` "End interaction with : " (`KismetSystemLibrary.GetDisplayName` self)))
  (`PrimitiveComponent.SetMaterial` (`self.CubeInteract`) 0 (`self.BaseMaterial`)))

(event `/Game/Features/Interactions/Component/BPI_Interactable.Hover`
  (`KismetSystemLibrary.PrintString` (`KismetStringLibrary.Concat_StrStr` "Hover : " (`KismetSystemLibrary.GetDisplayName` self)))
  (`PrimitiveComponent.SetMaterial` (`self.CubeHover`) 0 (`self.HoverMaterial`)))

(event `/Game/Features/Interactions/Component/BPI_Interactable.UnHover`
  (`KismetSystemLibrary.PrintString` (`KismetStringLibrary.Concat_StrStr` "UnHover  : " (`KismetSystemLibrary.GetDisplayName` self)))
  (`PrimitiveComponent.SetMaterial` (`self.CubeHover`) 0 (`self.BaseMaterial`)))

(event `self.ReceiveTick`
  (params (DeltaSeconds :type "Float (single-precision)"))
  (`parent.ReceiveTick` DeltaSeconds))

(event `/Game/Features/Interactions/Component/BPI_Interactable.UseItem`
  (`KismetSystemLibrary.PrintString` "UseItem1"))

(fn `UserConstructionScript`
  (`parent.UserConstructionScript`))